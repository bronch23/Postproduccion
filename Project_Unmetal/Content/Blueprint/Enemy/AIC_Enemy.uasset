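; AIC_Enemy is the AI controller for BP_Enemy pawns, driving their behavior through BT_Enemy and the BB_Enemy blackboard.
; On BeginPlay it sets up the blackboard, seeds NextPosition from the pawn's current waypoint, and runs the behavior tree.
; Helper functions write blackboard state: one flags the player as detected, one stores a Brother object reference, and one sets the Alarm flag.
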(event `self.ReceiveBeginPlay`
  (bind _blackboardcomponent (`self.UseBlackboard` "/Game/Blueprint/Enemy/BB_Enemy.BB_Enemy"))
  (bind _output_get (set `self.Blackboard Component` _blackboardcomponent))
  (`BlackboardComponent.SetValueAsVector` _output_get "NextPosition" (`/Game/Blueprint/Enemy/BP_Enemy.CurrentWP` (cast `/Game/Blueprint/Enemy/BP_Enemy` (`self.K2_GetPawn`) :!pure true)))
  (`self.RunBehaviorTree` "/Game/Blueprint/Enemy/BT_Enemy.BT_Enemy"))

(fn `Player Detected`
  (`BlackboardComponent.SetValueAsBool` (`self.Blackboard Component`) "PlayerDetected" true))

(fn `Set Alarm`
  (params (Alarm :type Boolean))
  (`BlackboardComponent.SetValueAsBool` (`self.Blackboard Component`) "Alarm" Alarm))

(fn `Set Brother`
  (params (Brother :type "/Game/Blueprint/Enemy/BP_Enemy Object Reference"))
  (`BlackboardComponent.SetValueAsObject` (`self.Blackboard Component`) "Brother" Brother))

(fn `UserConstructionScript`)