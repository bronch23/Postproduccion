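; BP_Enemy is an AI-controlled enemy that detects the player by sight and supplies patrol waypoints.
; PawnSensing sightings start a delayed check that notifies AIC_Enemy only if the player is still seen after the error margin.
; A retriggerable delay ends the sighting, records the player's last position and re-arms detection.
; Construction sets sight range and angle and transforms local waypoints to world space, which NextPoint cycles through.
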(event `self.ReceiveBeginPlay`
  (set `self.AI_Controller` (cast `/Game/Blueprint/Enemy/AIC_Enemy` (`AIBlueprintHelperLibrary.GetAIController` self) :!pure true)))

(event `self.PawnSensing.OnSeePawn`
  (params (Pawn :type "Pawn Object Reference"))
  (cast `/Game/FirstPerson/Blueprints/BP_FirstPersonCharacter` Pawn)
  (`|ExecutionSequence`
    (:`then_0`
      (set `self.SeeingPlayer` true)
      (`/Engine/EditorBlueprintResources/StandardMacros.DoOnce` false :!label _label
        (:`Completed`
          (`self.SightError`))))
    (:`then_1`
      (`KismetSystemLibrary.RetriggerableDelay` 0.6)
      (set `self.Player_LastPosition` (`self.K2_GetActorLocation` (`GameplayStatics.GetPlayerCharacter` 0)))
      (set `self.SeeingPlayer` false)
      (goto _label :!via `Reset`))))

(event `SightError`
  (`KismetSystemLibrary.Delay` (`self.SightErrorMargen`))
  (if (`self.SeeingPlayer`)
    (`/Game/Blueprint/Enemy/AIC_Enemy.Player Detected` (`self.AI_Controller`) true)))

(fn `NextPoint`
  (bind _transformedwaypoints (`self.TransformedWayPoints`))
  (if (not (< (`self.WPIndex`) (`KismetArrayLibrary.Array_Length` _transformedwaypoints)))
    (set `self.WPIndex` 0))
  (set `self.CurrentWP` (`|GetArrayItem` _transformedwaypoints (`self.WPIndex`)))
  (`/Engine/EditorBlueprintResources/StandardMacros.IncrementInt` (`self.WPIndex`)))

(fn `UserConstructionScript`
  (bind _pawnsensing (`self.PawnSensing`))
  (for (_ _array_index) (`self.WayPoints`)
    (`KismetArrayLibrary.Array_AddUnique` (`self.TransformedWayPoints`) (`KismetMathLibrary.TransformLocation` (`self.GetTransform`) (`|GetArrayItem` (`self.WayPoints`) _array_index)))
    (set `PawnSensingComponent.SightRadius` (`self.SightDistance`) _pawnsensing)
    (`PawnSensingComponent.SetPeripheralVisionAngle` _pawnsensing (`self.SightAngle`)))
  (set `self.CurrentWP` (`|GetArrayItem` (`self.TransformedWayPoints`) (`self.WPIndex`))))